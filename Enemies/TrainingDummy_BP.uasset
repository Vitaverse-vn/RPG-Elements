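; Training dummy enemy Blueprint that reacts to damage and elemental status effects.
; Any damage calls KillCheck on the player character, passing the dummy.
; Fire sets a status effect and attaches a fireball particle to the mesh.
; Ice sets a different status, destroying the flame emitter first if burning, while Shock is an empty stub.
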(event EventFire
  (Variables|Default|SetStatusEffect "NewEnumerator1")
  (bind _returnvalue (Effects|SpawnEmitterAttached "/Game/FXVarietyPack/Particles/P_ky_fireBall.P_ky_fireBall" (Variables|Character|GetMesh) "None"))
  (Variables|Default|SetEmitterFlame _returnvalue))

(event EventIce
  (bind _emitterflame (Variables|Default|GetEmitterFlame))
  (if (Utilities|Enum|Equal(Enum) (Variables|Default|GetStatusEffect) "NewEnumerator1")
    (Utilities|IsValid _emitterflame
      (:Is%20Valid
        (Components|DestroyComponent _emitterflame))))
  (Variables|Default|SetStatusEffect "NewEnumerator2"))

(event EventShock)

(event Game|Damage|EventAnyDamage
  (params (Damage :type Float%20%28single-precision%29) (DamageType :type Damage%20Type%20Object%20Reference) (InstigatedBy :type Controller%20Object%20Reference) (DamageCauser :type Actor%20Object%20Reference))
  (bind _asplayer_bp (Utilities|Casting|CastToPlayer_BP (Game|GetPlayerCharacter 0)))
  (Default|KillCheck _asplayer_bp "TrainingDummy_BP_C"))

(fn ConstructionScript)