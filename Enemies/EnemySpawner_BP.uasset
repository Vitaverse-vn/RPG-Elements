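; Enemy spawner actor that keeps up to a set number of random enemy types alive inside a box zone.
; A delayed loop starting at BeginPlay checks that it is active and the player is nearby, prunes invalid enemies, then spawns one with random yaw.
; A downward trace snaps each spawn toward the ground.
; A separate shutoff box pauses spawning while the player overlaps it; the construction script configures both boxes.
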(event OnComponentBeginOverlap(ShutoffZone)
  (params (OverlappedComponent :type Primitive%20Component%20Object%20Reference) (OtherActor :type Actor%20Object%20Reference) (OtherComp :type Primitive%20Component%20Object%20Reference) (OtherBodyIndex :type Integer) (bFromSweep :type Boolean) (SweepResult :type Hit%20Result%20Structure%20%28by%20ref%29))
  (Utilities|Casting|CastToPlayer_BP OtherActor)
  (Variables|Default|SetActive? false))

(event OnComponentEndOverlap(ShutoffZone)
  (params (OverlappedComponent :type Primitive%20Component%20Object%20Reference) (OtherActor :type Actor%20Object%20Reference) (OtherComp :type Primitive%20Component%20Object%20Reference) (OtherBodyIndex :type Integer))
  (Utilities|Casting|CastToPlayer_BP OtherActor)
  (Variables|Default|SetActive? true))

(event Custom|SpawnCheck
  (bind _spawnzone (Variables|Default|GetSpawnZone))
  (bind _enemiesspawned (Variables|Default|GetEnemiesSpawned))
  (if (and (Variables|Default|GetActive?) (< (Transformation|GetDistanceTo (Game|GetPlayerCharacter 0)) 1e+04))
    (for _array_element _enemiesspawned
      (Utilities|IsValid _array_element
        (:Is%20Not%20Valid
          (Utilities|Array|RemoveItem (Variables|Default|GetEnemiesSpawned) _array_element))))
    (if (>= (Utilities|Array|Length _enemiesspawned) (Variables|Default|GetEnemyAmount))
      _
      (else
        (bind _returnvalue (Game|SpawnActorfromClass (.OutItem (Utilities|Array|Random (Variables|Default|GetEnemiesToSpawn))) (Math|Transform|MakeTransform (Math|Random|RandomPointinBoundingBox (Transformation|GetWorldLocation _spawnzone) (Components|Box|GetScaledBoxExtent _spawnzone)) (Math|Rotator|MakeRotator 0.0 0.0 (Math|Random|RandomFloatinRange -1.8e+02 1.8e+02)) "1.000000,1.000000,1.000000") "Undefined" 0 0))
        (Utilities|IsValid _returnvalue
          (:Is%20Valid
            (Utilities|Array|AddUnique (Variables|Default|GetEnemiesSpawned) _returnvalue)
            (bind _output_get (Variables|Default|SetSpawnerUnit _returnvalue))
            (bind (_outhit _returnvalue_2) (Collision|LineTraceByChannel (- (Transformation|GetActorLocation _returnvalue) "0,0,100.000000") (- (Transformation|GetActorLocation _returnvalue) "0,0,500.000000") "TraceTypeQuery1" false (Utilities|Array|MakeArray _output_get) "None"))
            (if _returnvalue_2
              (Transformation|SetActorLocation (Variables|Default|GetSpawnerUnit) (+ (.Location (Collision|BreakHitResult _outhit)) "0,0,90.000000") false false)))
          (:Is%20Not%20Valid
            _)))))
  (Utilities|FlowControl|Delay (Variables|Default|GetSpawnDelay))
  (CallFunction|SpawnCheck))

(event EventBeginPlay
  (bind _spawnzone (Variables|Default|GetSpawnZone))
  (bind _enemiesspawned (Variables|Default|GetEnemiesSpawned))
  (if (and (Variables|Default|GetActive?) (< (Transformation|GetDistanceTo (Game|GetPlayerCharacter 0)) 1e+04))
    (for _array_element _enemiesspawned
      (Utilities|IsValid _array_element
        (:Is%20Not%20Valid
          (Utilities|Array|RemoveItem (Variables|Default|GetEnemiesSpawned) _array_element))))
    (if (>= (Utilities|Array|Length _enemiesspawned) (Variables|Default|GetEnemyAmount))
      _
      (else
        (bind _returnvalue (Game|SpawnActorfromClass (.OutItem (Utilities|Array|Random (Variables|Default|GetEnemiesToSpawn))) (Math|Transform|MakeTransform (Math|Random|RandomPointinBoundingBox (Transformation|GetWorldLocation _spawnzone) (Components|Box|GetScaledBoxExtent _spawnzone)) (Math|Rotator|MakeRotator 0.0 0.0 (Math|Random|RandomFloatinRange -1.8e+02 1.8e+02)) "1.000000,1.000000,1.000000") "Undefined" 0 0))
        (Utilities|IsValid _returnvalue
          (:Is%20Valid
            (Utilities|Array|AddUnique (Variables|Default|GetEnemiesSpawned) _returnvalue)
            (bind _output_get (Variables|Default|SetSpawnerUnit _returnvalue))
            (bind (_outhit _returnvalue_2) (Collision|LineTraceByChannel (- (Transformation|GetActorLocation _returnvalue) "0,0,100.000000") (- (Transformation|GetActorLocation _returnvalue) "0,0,500.000000") "TraceTypeQuery1" false (Utilities|Array|MakeArray _output_get) "None"))
            (if _returnvalue_2
              (Transformation|SetActorLocation (Variables|Default|GetSpawnerUnit) (+ (.Location (Collision|BreakHitResult _outhit)) "0,0,90.000000") false false)))
          (:Is%20Not%20Valid
            _)))))
  (Utilities|FlowControl|Delay (Variables|Default|GetSpawnDelay))
  (CallFunction|SpawnCheck))

(fn ConstructionScript
  (bind _shutoffzone (Variables|Default|GetShutoffZone))
  (Components|Box|SetBoxExtent (Variables|Default|GetSpawnZone) (Variables|Default|GetSpawnZoneSize) true)
  (Components|Box|SetBoxExtent _shutoffzone (Variables|Default|GetShutOffZoneSize) true)
  (Transformation|SetRelativeLocation _shutoffzone (Variables|Default|GetShutOffZoneLocation) false false))