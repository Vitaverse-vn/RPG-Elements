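; Base enemy character that roams, fights or flees from the player, then leaves loot on death.
; A behavior-mode switch runs AIMoveTo patrol, chase and flee loops, with pawn sensing or damage starting a chase and a polled range check ending it.
; Montage notifies trigger sphere-trace attacks.
; Death grants XP, reports the kill and rolls loot, which the player previews on the HUD and takes on a second interact.
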(event OnSeePawn(PawnSensing)
  (params (Pawn :type Pawn%20Object%20Reference))
  (bind _self self)
  ;[1 1 1] When Enemy See The Player
  (if (not (Variables|Default|GetDead?))
    (if (Variables|Default|GetPassive?)
      (if (Variables|Default|GetTimid?)
        (Variables|Default|SetBehaviorMode "NewEnumerator4")
        (Variables|Default|SetScared? true)
        (CallFunction|BehaviorUnit))
      (else
        (bind _asplayer_bp (Utilities|Casting|CastToPlayer_BP Pawn))
        (Variables|Default|SetPlayer_Ref _asplayer_bp)
        ;[1 1 1] You can see Enemy's Health
        (Utilities|FlowControl|DoOnce false
          (:Completed
            (Variables|Default|SetStartPoint (Transformation|GetActorLocation))
            (Variables|/Script/Engine.CharacterMovementComponent|SetMaxWalkSpeed (Variables|Character|GetCharacterMovement) (Variables|Default|GetChaseSpeed))
            (Utilities|Array|AddUnique (Variables|/Game/ThirdPerson/Blueprints/Player_BP.Player_BP_C|GetEnemyList (Variables|Default|GetPlayer_Ref)) _self)
            (bind _returnvalue (UserInterface|CreateWidget "/Game/ThirdPerson/Blueprints/HUD_Elements/EnemyList_UI.EnemyList_UI_C" 0 _self))
            (bind _output_get (Variables|Default|SetAI_Health_WBP _returnvalue))
            (Widget|Panel|AddChild (Variables|/Game/ThirdPerson/Blueprints/HUD_Elements/PlayerHUD_WBP.PlayerHUD_WBP_C|GetEnemyList (Variables|/Game/ThirdPerson/Blueprints/Player_BP.Player_BP_C|GetPlayerHUD_Ref (Variables|Default|GetPlayer_Ref))) _output_get)
            (Variables|Default|SetAttackTarget (Variables|Default|GetPlayer_Ref))
            (Variables|Default|SetBehaviorMode "NewEnumerator2")
            (CallFunction|BehaviorUnit)
            (CallFunction|DisengageCheck)))))))

(event OnComponentBeginOverlap(InteractRadius)
  (params (OverlappedComponent :type Primitive%20Component%20Object%20Reference) (OtherActor :type Actor%20Object%20Reference) (OtherComp :type Primitive%20Component%20Object%20Reference) (OtherBodyIndex :type Integer) (bFromSweep :type Boolean) (SweepResult :type Hit%20Result%20Structure%20%28by%20ref%29))
  ;[1 1 1] Radius that we can loot Items from Enemy
  (bind _asplayer_bp (Utilities|Casting|CastToPlayer_BP OtherActor))
  (if (Variables|Default|GetDead?)
    (Utilities|Array|AddUnique (Variables|/Game/ThirdPerson/Blueprints/Player_BP.Player_BP_C|GetInteractable_InRange _asplayer_bp) self)))

(event OnComponentEndOverlap(InteractRadius)
  (params (OverlappedComponent :type Primitive%20Component%20Object%20Reference) (OtherActor :type Actor%20Object%20Reference) (OtherComp :type Primitive%20Component%20Object%20Reference) (OtherBodyIndex :type Integer))
  ;[1 1 1] Radius that we can loot Items from Enemy
  (bind _asplayer_bp (Utilities|Casting|CastToPlayer_BP OtherActor))
  (if (Utilities|Array|ContainsItem (Variables|/Game/ThirdPerson/Blueprints/Player_BP.Player_BP_C|GetInteractable_InRange _asplayer_bp) self)
    (Utilities|Array|RemoveItem (Variables|/Game/ThirdPerson/Blueprints/Player_BP.Player_BP_C|GetInteractable_InRange _asplayer_bp) _asplayer_bp)))

(event Custom|BehaviorUnit
  (bind _charactermovement (Variables|Character|GetCharacterMovement))
  ;[1 1 1] AI Behavior
  (if (not (Variables|Default|GetDead?))
    (switch Utilities|FlowControl|Switch|SwitchonBehaviorModes (Variables|Default|GetBehaviorMode)
      (:NewEnumerator0
        ;[1 1 1] Roam
        (AI|AIMoveTo self (.RandomLocation (AI|Navigation|GetRandomReachablePointinRadius (Transformation|GetActorLocation) (Variables|Default|GetRoamRadius) 0 0)) 0 5.0 false
          (:OnSuccess
            (CallFunction|UpdatePatrolPoint)
            (Utilities|FlowControl|Delay (Math|Random|RandomFloatinRange (Variables|Default|GetMinWait) (Variables|Default|GetMaxWait)))
            (if (Variables|Default|GetScared?)
              (CallFunction|Flee :!label _label)
              (elif (Utilities|Enum|Equal(Enum) (Variables|Default|GetBehaviorMode) "NewEnumerator2")
                (CallFunction|ChasePlayer)
                (else
                  (Variables|Default|SetBehaviorMode "NewEnumerator1")
                  (CallFunction|BehaviorUnit)))))))
      (:NewEnumerator1
        (AI|AIMoveTo self "0, 0, 0" (Variables|Default|GetPatrolPoint) 5.0 false
          (:OnSuccess
            (Utilities|FlowControl|Delay (Math|Random|RandomFloatinRange (Variables|Default|GetMinWait) (Variables|Default|GetMaxWait)))
            (if (Variables|Default|GetScared?)
              (goto _label)
              (elif (Utilities|Enum|Equal(Enum) (Variables|Default|GetBehaviorMode) "NewEnumerator2")
                (CallFunction|ChasePlayer)
                (else
                  (Variables|Default|SetBehaviorMode "NewEnumerator0")
                  (CallFunction|BehaviorUnit)))))))
      (:NewEnumerator2
        ;[1 1 1] Chase Player
        (if (not (Variables|Default|GetDead?))
          (AI|AIMoveTo self "0, 0, 0" (Variables|Default|GetAttackTarget) (Variables|Default|GetAttackAcceptanceRadius) false
            (:OnSuccess
              (Utilities|FlowControl|DoOnce false
                (:Completed
                  (Variables|Default|SetAttackingPlayer? true)
                  (bind _notifyname (Animation|Montage|PlayMontage (Variables|Character|GetMesh) (Utilities|Select :Index (Math|Random|RandomInteger (Variables|Default|GetEnemyAttackAmount)) :Option%200 (Variables|Default|GetATK_Montage) :Option%201 (Variables|Default|GetAttack_02) :Option%202 (Variables|Default|GetAttack_03) :Option%203 (Variables|Default|GetAttack_04)))
                    (:then
                      (Components|Movement|StopMovementImmediately _charactermovement)
                      (Variables|/Script/Engine.CharacterMovementComponent|SetMaxWalkSpeed _charactermovement 0.0)
                      (CallFunction|TrackPlayer))
                    (:OnCompleted
                      (Utilities|FlowControl|Delay (Math|Random|RandomFloatinRange 0.1 0.3))
                      (Variables|Default|SetAttackingPlayer? false)
                      (if (not (Variables|Default|GetDead?))
                        (CallFunction|ReleaseATK)
                        (Variables|/Script/Engine.CharacterMovementComponent|SetMaxWalkSpeed (Variables|Character|GetCharacterMovement) 6e+02)
                        (CallFunction|BehaviorUnit)))
                    (:OnNotifyBegin
                      (switch name _notifyname
                        (:AttackTrace
                          (CallFunction|AttackTrace)))))))))))
      (:NewEnumerator4
        ;[1 1 1] Flee
        (Variables|Default|SetBehaviorMode "NewEnumerator4")
        (CallFunction|Flee)))))

(event Custom|ChasePlayer
  (bind _charactermovement (Variables|Character|GetCharacterMovement))
  ;[1 1 1] Chase Player
  (if (not (Variables|Default|GetDead?))
    (AI|AIMoveTo self "0, 0, 0" (Variables|Default|GetAttackTarget) (Variables|Default|GetAttackAcceptanceRadius) false
      (:OnSuccess
        (Utilities|FlowControl|DoOnce false
          (:Completed
            (Variables|Default|SetAttackingPlayer? true)
            (bind _notifyname (Animation|Montage|PlayMontage (Variables|Character|GetMesh) (Utilities|Select :Index (Math|Random|RandomInteger (Variables|Default|GetEnemyAttackAmount)) :Option%200 (Variables|Default|GetATK_Montage) :Option%201 (Variables|Default|GetAttack_02) :Option%202 (Variables|Default|GetAttack_03) :Option%203 (Variables|Default|GetAttack_04)))
              (:then
                (Components|Movement|StopMovementImmediately _charactermovement)
                (Variables|/Script/Engine.CharacterMovementComponent|SetMaxWalkSpeed _charactermovement 0.0)
                (CallFunction|TrackPlayer))
              (:OnCompleted
                (Utilities|FlowControl|Delay (Math|Random|RandomFloatinRange 0.1 0.3))
                (Variables|Default|SetAttackingPlayer? false)
                (if (not (Variables|Default|GetDead?))
                  (CallFunction|ReleaseATK)
                  (Variables|/Script/Engine.CharacterMovementComponent|SetMaxWalkSpeed (Variables|Character|GetCharacterMovement) 6e+02)
                  (CallFunction|BehaviorUnit)))
              (:OnNotifyBegin
                (switch name _notifyname
                  (:AttackTrace
                    (CallFunction|AttackTrace)))))))))))

(event Custom|Damaged
  (bind _self self)
  (Utilities|FlowControl|DoOnce false
    (:Completed
      (bind _asplayer_bp (Utilities|Casting|CastToPlayer_BP (stale OnSeePawn(PawnSensing) Pawn)))
      (Variables|Default|SetPlayer_Ref _asplayer_bp)
      ;[1 1 1] You can see Enemy's Health
      (Utilities|FlowControl|DoOnce false
        (:Completed
          (Variables|Default|SetStartPoint (Transformation|GetActorLocation))
          (Variables|/Script/Engine.CharacterMovementComponent|SetMaxWalkSpeed (Variables|Character|GetCharacterMovement) (Variables|Default|GetChaseSpeed))
          (Utilities|Array|AddUnique (Variables|/Game/ThirdPerson/Blueprints/Player_BP.Player_BP_C|GetEnemyList (Variables|Default|GetPlayer_Ref)) _self)
          (bind _returnvalue (UserInterface|CreateWidget "/Game/ThirdPerson/Blueprints/HUD_Elements/EnemyList_UI.EnemyList_UI_C" 0 _self))
          (bind _output_get (Variables|Default|SetAI_Health_WBP _returnvalue))
          (Widget|Panel|AddChild (Variables|/Game/ThirdPerson/Blueprints/HUD_Elements/PlayerHUD_WBP.PlayerHUD_WBP_C|GetEnemyList (Variables|/Game/ThirdPerson/Blueprints/Player_BP.Player_BP_C|GetPlayerHUD_Ref (Variables|Default|GetPlayer_Ref))) _output_get)
          (Variables|Default|SetAttackTarget (Variables|Default|GetPlayer_Ref))
          (Variables|Default|SetBehaviorMode "NewEnumerator2")
          (CallFunction|BehaviorUnit)
          (CallFunction|DisengageCheck))))))

(event Custom|ReleaseATK
  (bind _charactermovement (Variables|Character|GetCharacterMovement))
  ;[1 1 1] Chase Player
  (Utilities|FlowControl|DoOnce false) ; enters at Reset
)

(event Custom|TrackPlayer
  ;[1 1 1] Track Player when they see
  (Variables|Default|GetAttackTarget
    (:then
      (if (Variables|Default|GetAttackingPlayer?)
        (Transformation|SetActorRotation (Math|Rotator|MakeRotator 0.0 0.0 (.yaw (Math|Rotator|FindLookatRotation (Transformation|GetActorLocation) (Transformation|GetActorLocation (Variables|Default|GetAttackTarget))))))
        (Utilities|FlowControl|Delay 0.01)
        (CallFunction|TrackPlayer)))
    (:else)))

(event Custom|DisengageCheck
  ;[1 1 1] If Player out chase range, Enemy stop aatack
  (bind _player_ref (Variables|Default|GetPlayer_Ref)
    (:then
      (if (>= (Transformation|GetDistanceTo _player_ref 0) (Variables|Default|GetChaseRange))
        (Variables|Default|SetAttackingPlayer? false)
        (Variables|Default|SetBehaviorMode "NewEnumerator0")
        (AI|AIMoveTo self (Variables|Default|GetStartPoint) 0 5.0 false
          (:then
            (Class|PanelWidget|RemoveChild (Variables|/Game/ThirdPerson/Blueprints/HUD_Elements/PlayerHUD_WBP.PlayerHUD_WBP_C|GetEnemyList (Variables|/Game/ThirdPerson/Blueprints/Player_BP.Player_BP_C|GetPlayerHUD_Ref (Variables|Default|GetPlayer_Ref))) (Variables|Default|GetAI_Health_WBP))
            (CallFunction|Reset))
          (:OnSuccess
            (Utilities|FlowControl|Delay 0.2)
            (CallFunction|BehaviorUnit)
            (Variables|/Script/Engine.CharacterMovementComponent|SetMaxWalkSpeed (Variables|Character|GetCharacterMovement) (Variables|Default|GetWalkSpeed))))
        (else
          (Utilities|FlowControl|Delay 0.2)
          (CallFunction|DisengageCheck))))
    (:else)))

(event Custom|Reset
  (bind _self self)
  (Utilities|FlowControl|Sequence
    (:then_0
      (Utilities|FlowControl|DoOnce false) ; enters at Reset
    )
    (:then_1
      ;[1 1 1] You can see Enemy's Health
      (Utilities|FlowControl|DoOnce false) ; enters at Reset
    )))

(event Custom|Flee
  (bind _returnvalue (Transformation|GetActorLocation))
  (bind _returnvalue_2 (Game|GetPlayerCharacter 0))
  (bind _returnvalue_3 (Transformation|GetActorLocation _returnvalue_2))
  (bind _returnvalue_4 (Math|Rotator|FindLookatRotation _returnvalue _returnvalue_3))
  (bind _returnvalue_5 (Math|Vector|GetForwardVector _returnvalue_4))
  (bind _returnvalue_6 (* _returnvalue_5 -5e+02))
  (bind _returnvalue_7 (+ _returnvalue _returnvalue_6))
  (bind (_x _y) (Math|Vector|BreakVector _returnvalue_7))
  ;[1 1 1] Flee
  (if (not (Variables|Default|GetDead?))
    (AI|AIMoveTo self (.RandomLocation (AI|Navigation|GetRandomReachablePointinRadius (Math|Vector|MakeVector _x _y (.Z (Math|Vector|BreakVector _returnvalue))) 5e+02 0 0)) 0 5.0 false
      (:OnSuccess
        _)
      (:OnFail
        _))
    (CallFunction|Flee)))

(event Custom|Looted
  (bind _self self)
  (bind _player_ref (Variables|Default|GetPlayer_Ref))
  (bind _interactable_inrange (Variables|/Game/ThirdPerson/Blueprints/Player_BP.Player_BP_C|GetInteractable_InRange _player_ref))
  ;[1 1 1] Looted
  (bind _lootsystem (Variables|Default|GetLootSystem)
    (:then
      (Components|DestroyComponent _lootsystem))
    (:else
      _))
  (Utilities|FlowControl|Delay 5.0)
  (if (Utilities|Array|ContainsItem _interactable_inrange _self)
    (Utilities|Array|RemoveItem _interactable_inrange _self))
  (Actor|DestroyActor))

(event EventBeginPlay
  ;[1 1 1] Event Begin Play
  (CallFunction|BehaviorUnit))

(event Game|Damage|EventAnyDamage
  (params (Damage :type Float%20%28single-precision%29) (DamageType :type Damage%20Type%20Object%20Reference) (InstigatedBy :type Controller%20Object%20Reference) (DamageCauser :type Actor%20Object%20Reference))
  (bind _self self)
  (bind _mesh (Variables|Character|GetMesh))
  (bind _returnvalue (Components|SkeletalMesh|GetAnimInstance _mesh))
  ;[1 1 1] Enemy Damaged
  (Utilities|Casting|CastToPlayer_BP DamageCauser)
  (if true
    (Variables|Default|GetPlayer_Ref
      (:then
        _)
      (:else
        (bind _asplayer_bp (Utilities|Casting|CastToPlayer_BP DamageCauser))
        (Variables|Default|SetPlayer_Ref _asplayer_bp)))
    (bind _output_get (Variables|Default|SetHealth (- (Variables|Default|GetHealth) Damage)))
    ;[1 1 1] Enemy Dead
    (if (<= _output_get 0.0)
      (Utilities|FlowControl|DoOnce false
        (:Completed
          (Variables|Default|SetDead? true)
          ;[1 1 1] Gain XP From Enemy
          (bind _player_ref (Variables|Default|GetPlayer_Ref)
            (:then
              _)
            (:else
              (bind _asplayer_bp_2 (Utilities|Casting|CastToPlayer_BP (Game|GetPlayerCharacter 0)))
              (bind _output_get_2 (Variables|Default|SetPlayer_Ref _asplayer_bp_2))))
          (Default|GainXP _player_ref (Variables|Default|GetXPValue))
          (Default|KillCheck _output_get_2 (Utilities|GetClass self))
          ;[1 1 1] Loot Items
          (if (Variables|Default|GetSkinnable?)
            (Utilities|Array|AddUnique (Variables|Default|GetActualLoot) (Variables|Default|GetSkinID)))
          (CallFunction|DropLootCheck)
          (Components|Movement|StopMovementImmediately (Variables|Character|GetCharacterMovement))
          (if (Class|AnimInstance|IsAnyMontagePlaying _returnvalue)
            (Animation|Montage|MontageStop _returnvalue 0.0 (Animation|Montage|GetCurrentActiveMontage _returnvalue)))
          (Variables|/Script/Engine.CharacterMovementComponent|SetMaxWalkSpeed (Variables|Character|GetCharacterMovement) 0.0)
          (Variables|Default|SetAttackingPlayer? false)
          (Variables|Default|SetBehaviorMode "NewEnumerator3")
          (CallFunction|BehaviorUnit)
          (Class|PanelWidget|RemoveChild (Variables|/Game/ThirdPerson/Blueprints/HUD_Elements/PlayerHUD_WBP.PlayerHUD_WBP_C|GetEnemyList (Variables|/Game/ThirdPerson/Blueprints/Player_BP.Player_BP_C|GetPlayerHUD_Ref (Variables|Default|GetPlayer_Ref))) (Variables|Default|GetAI_Health_WBP))
          (Collision|SetCollisionResponsetoChannel (Variables|Character|GetMesh) "ECC_Visibility" "ECR_Ignore")
          (Collision|SetCollisionResponsetoChannel (Variables|Character|GetMesh) "ECC_Pawn" "ECR_Ignore")
          ;[1 1 1] Looted Item
          (if (not (> (Utilities|Array|Length (Variables|Default|GetActualLoot)) 0))
            (CallFunction|Looted)
            (if (Utilities|Array|ContainsItem (Variables|/Game/ThirdPerson/Blueprints/Player_BP.Player_BP_C|GetInteractable_InRange (Variables|Default|GetPlayer_Ref)) _self)
              (Utilities|Array|RemoveItem (Variables|/Game/ThirdPerson/Blueprints/Player_BP.Player_BP_C|GetInteractable_InRange (Variables|Default|GetPlayer_Ref)) _self)))))
      (else
        (CallFunction|Damaged)))))

(event EventHurt
  (bind _self self)
  ;[1 1 1] When Enemy get damaged, they start to attack Player
  (Utilities|FlowControl|DoOnce false
    (:Completed
      (bind _asplayer_bp (Utilities|Casting|CastToPlayer_BP (Game|GetPlayerCharacter 0)))
      (Variables|Default|SetPlayer_Ref _asplayer_bp)
      (if (not (Variables|Default|GetTimid?))
        ;[1 1 1] You can see Enemy's Health
        (Utilities|FlowControl|DoOnce false
          (:Completed
            (Variables|Default|SetStartPoint (Transformation|GetActorLocation))
            (Variables|/Script/Engine.CharacterMovementComponent|SetMaxWalkSpeed (Variables|Character|GetCharacterMovement) (Variables|Default|GetChaseSpeed))
            (Utilities|Array|AddUnique (Variables|/Game/ThirdPerson/Blueprints/Player_BP.Player_BP_C|GetEnemyList (Variables|Default|GetPlayer_Ref)) _self)
            (bind _returnvalue (UserInterface|CreateWidget "/Game/ThirdPerson/Blueprints/HUD_Elements/EnemyList_UI.EnemyList_UI_C" 0 _self))
            (bind _output_get (Variables|Default|SetAI_Health_WBP _returnvalue))
            (Widget|Panel|AddChild (Variables|/Game/ThirdPerson/Blueprints/HUD_Elements/PlayerHUD_WBP.PlayerHUD_WBP_C|GetEnemyList (Variables|/Game/ThirdPerson/Blueprints/Player_BP.Player_BP_C|GetPlayerHUD_Ref (Variables|Default|GetPlayer_Ref))) _output_get)
            (Variables|Default|SetAttackTarget (Variables|Default|GetPlayer_Ref))
            (Variables|Default|SetBehaviorMode "NewEnumerator2")
            (CallFunction|BehaviorUnit)
            (CallFunction|DisengageCheck)))))))

(event EventInteract
  ;[1 1 1] Show what Items you looted from Enemy
  (bind _asplayer_bp (Utilities|Casting|CastToPlayer_BP (Game|GetPlayerCharacter 0)))
  (if (Class|PanelWidget|HasAnyChildren (Variables|/Game/ThirdPerson/Blueprints/HUD_Elements/PlayerHUD_WBP.PlayerHUD_WBP_C|GetLootTable (Variables|/Game/ThirdPerson/Blueprints/Player_BP.Player_BP_C|GetPlayerHUD_Ref _asplayer_bp)))
    (CallFunction|TakeAll)
    (Widget|Panel|ClearChildren (Variables|/Game/ThirdPerson/Blueprints/HUD_Elements/PlayerHUD_WBP.PlayerHUD_WBP_C|GetLootTable (Variables|/Game/ThirdPerson/Blueprints/Player_BP.Player_BP_C|GetPlayerHUD_Ref _asplayer_bp)))
    (Utilities|Array|Clear (Variables|Default|GetActualLoot))
    (CallFunction|Looted)
    (else
      (for _array_element (Variables|Default|GetActualLoot)
        (bind _returnvalue (Utilities|GetDataTableRow "/Game/ThirdPerson/Blueprints/InteractionSystem/ItemsInfo_DataTB.ItemsInfo_DataTB" (Utilities|String|StringToName (Utilities|String|EnumtoString _array_element)))
          (:then
            (bind _returnvalue_2 (UserInterface|CreateWidget "/Game/ThirdPerson/Blueprints/HUD_Elements/LootIcon_UI.LootIcon_UI_C" 0 _returnvalue self))
            (Class|VerticalBox|AddChildtoVerticalBox (Variables|/Game/ThirdPerson/Blueprints/HUD_Elements/PlayerHUD_WBP.PlayerHUD_WBP_C|GetLootTable (Variables|/Game/ThirdPerson/Blueprints/Player_BP.Player_BP_C|GetPlayerHUD_Ref _asplayer_bp)) _returnvalue_2)))))))

(fn ConstructionScript
  (bind _self self)
  (bind _outactors (Actor|GetAllActorsOfClass "/Game/ThirdPerson/Blueprints/Characters/Enemies/EnemyPatrolPoint_BP.EnemyPatrolPoint_BP_C"))
  (Variables|Default|SetPatrolPoint (Utilities|Array|Get(acopy) _outactors))
  (for _array_element _outactors
    (if (< (Transformation|GetDistanceTo _array_element _self) (Transformation|GetDistanceTo (Variables|Default|GetPatrolPoint) _self))
      (Variables|Default|SetPatrolPoint _array_element))))

(fn UpdatePatrolPoint
  (bind _self self)
  (bind _outactors (Actor|GetAllActorsOfClass "/Game/ThirdPerson/Blueprints/Characters/Enemies/EnemyPatrolPoint_BP.EnemyPatrolPoint_BP_C"))
  (for _array_element _outactors
    (if (< (Transformation|GetDistanceTo _array_element _self) (Transformation|GetDistanceTo (Variables|Default|GetPatrolPoint) _self))
      (Variables|Default|SetPatrolPoint _array_element))))

(fn AttackTrace
  (bind _returnvalue (Transformation|GetActorLocation))
  (bind _atk_damage (Variables|Default|GetATK_Damage))
  (bind _random_damage (Variables|Default|GetRandom%20Damage))
  (bind (_outhit _returnvalue_2) (Collision|SphereTraceByChannel _returnvalue (+ _returnvalue (* (Transformation|GetActorForwardVector) (Variables|Default|GetATK%20Range))) (Variables|Default|GetATK%20Radius) "TraceTypeQuery3" false 0 "None"))
  (if _returnvalue_2
    (Game|Damage|ApplyDamage (.HitActor (Collision|BreakHitResult _outhit)) (Math|Conversions|ToFloat(Integer) (Math|Float|Round (Math|Random|RandomFloatinRange (- _atk_damage _random_damage) (+ _atk_damage _random_damage)))) 0 0)))

(fn DropLootCheck
  (bind _returnvalue (Transformation|GetActorTransform))
  (for _array_element (Variables|Default|GetPotentialLoot)
    (if (>= (Math|Random|RandomIntegerinRange 0 100) (Variables|Default|GetDropChance))
      (Utilities|Array|AddUnique (Variables|Default|GetActualLoot) _array_element)))
  (if (> (Utilities|Array|Length (Variables|Default|GetActualLoot)) 0)
    (bind _returnvalue_2 (Effects|SpawnEmitteratLocation "/Game/FXVarietyPack/Particles/P_ky_fireBall.P_ky_fireBall" (.location _returnvalue) (.rotation _returnvalue)))
    (Variables|Default|SetLootSystem _returnvalue_2)))

(fn TakeAll
  (for _array_element (Variables|Default|GetActualLoot)
    (bind _returnvalue (Utilities|GetDataTableRow "/Game/ThirdPerson/Blueprints/InteractionSystem/ItemsInfo_DataTB.ItemsInfo_DataTB" (Utilities|String|StringToName (Utilities|String|EnumtoString _array_element)))
      (:then
        (Default|PickupItem (Variables|Default|GetPlayer_Ref) _returnvalue)))))