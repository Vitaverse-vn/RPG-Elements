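; FastTravelPoint_BP is an interactable fast travel point that the player discovers by walking into its sphere.
; On first overlap it adds itself to Player_BP's FastTravelPoint array and activates its particle system, which the Relight event can also reactivate.
; Interact toggles a FastTravel_WBP widget, created once and reused, switching input mode and mouse cursor visibility as it opens and closes.
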(event OnComponentBeginOverlap(Sphere)
  (params (OverlappedComponent :type Primitive%20Component%20Object%20Reference) (OtherActor :type Actor%20Object%20Reference) (OtherComp :type Primitive%20Component%20Object%20Reference) (OtherBodyIndex :type Integer) (bFromSweep :type Boolean) (SweepResult :type Hit%20Result%20Structure%20%28by%20ref%29))
  (bind _self self)
  (bind _asplayer_bp (Utilities|Casting|CastToPlayer_BP OtherActor))
  (if (not (Utilities|Array|ContainsItem (Variables|/Game/ThirdPerson/Blueprints/Player_BP.Player_BP_C|GetFastTravelPoint _asplayer_bp) _self))
    (Utilities|Array|AddUnique (Variables|/Game/ThirdPerson/Blueprints/Player_BP.Player_BP_C|GetFastTravelPoint _asplayer_bp) _self)
    (Components|Activation|Activate (Variables|Default|GetParticleSystem) false)))

(event Custom|Relight
  (Components|Activation|Activate (Variables|Default|GetParticleSystem) false))

(event EventInteract
  (bind _returnvalue (Game|GetPlayerController 0))
  (bind _returnvalue_2 (Game|GetPlayerController 0))
  (if (Variables|Default|GetOpen?)
    (Widget|RemovefromParent (Variables|Default|GetFastTravel_WBP))
    (Variables|Default|SetOpen? false)
    (Input|SetInputModeGameOnly _returnvalue_2)
    (Variables|/Script/Engine.PlayerController|SetbShowMouseCursor _returnvalue_2 false)
    (else
      (Utilities|IsValid (Variables|Default|GetFastTravel_WBP)
        (:Is%20Valid
          _)
        (:Is%20Not%20Valid
          (bind _returnvalue_3 (UserInterface|CreateWidget "/Game/ThirdPerson/Blueprints/InteractionSystem/FastTravelSystem/FastTravel_WBP.FastTravel_WBP_C"))
          (bind _output_get (Variables|Default|SetFastTravel_WBP _returnvalue_3))))
      (UserInterface|Viewport|AddtoViewport _output_get 0)
      (Variables|Default|SetOpen? true)
      (Input|SetInputModeGameandUI _returnvalue _output_get "DoNotLock" true)
      (Variables|/Script/Engine.PlayerController|SetbShowMouseCursor _returnvalue true))))

(fn ConstructionScript
  (|CallParentFunction))