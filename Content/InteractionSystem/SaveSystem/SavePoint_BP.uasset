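; SavePoint_BP is an interactable save statue that toggles a save screen when the player interacts with it.
; Opening creates SaveScreen_WBP with a reference back to the statue, shows the cursor, switches to Game and UI input, and copies its SaveLocation to Player_BP.
; Interacting again removes the widget and restores game-only input with the cursor hidden.
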(event EventInteract
  (bind _returnvalue (Game|GetPlayerController 0))
  (bind _returnvalue_2 (Game|GetPlayerController 0))
  (if (Variables|Default|GetSaveScreenOpen?)
    (Widget|RemovefromParent (Variables|Default|GetSaveScreen_Ref))
    (Variables|/Script/Engine.PlayerController|SetbShowMouseCursor _returnvalue_2 false)
    (Input|SetInputModeGameOnly _returnvalue_2)
    (Variables|Default|SetSaveScreenOpen? false)
    (else
      (bind _returnvalue_3 (UserInterface|CreateWidget "/Game/ThirdPerson/Blueprints/InteractionSystem/SaveSystem/SaveScreen_WBP.SaveScreen_WBP_C"))
      (Variables|/Game/ThirdPerson/Blueprints/InteractionSystem/SaveSystem/SaveScreen_WBP.SaveScreen_WBP_C|SetSaveStatue_Ref _returnvalue_3 self)
      (bind _output_get (Variables|Default|SetSaveScreen_Ref _returnvalue_3))
      (UserInterface|Viewport|AddtoViewport _output_get 0)
      (Variables|/Script/Engine.PlayerController|SetbShowMouseCursor _returnvalue true)
      (Input|SetInputModeGameandUI _returnvalue (Variables|Default|GetSaveScreen_Ref) "DoNotLock" true)
      (Variables|Default|SetSaveScreenOpen? true)
      (bind _asplayer_bp (Utilities|Casting|CastToPlayer_BP (Game|GetPlayerCharacter 0)))
      (Variables|/Game/ThirdPerson/Blueprints/Player_BP.Player_BP_C|SetSaveLocation _asplayer_bp (Variables|Default|GetSave_Location)))))

(fn ConstructionScript
  (|CallParentFunction))