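; Quest-giver actor that offers prerequisite-gated quests and shows a "!" or "?" text marker above available or accepted ones.
; BeginPlay filters its quest list through Quest_DataTable prerequisites and the player's completed quests, then Compare sets the marker from accepted quests.
; Interact toggles a reusable quest screen widget with cursor and input-mode switching.
; Closing it calls ReCheck on every QuestGiver_BP, restoring SavedQuests and rerunning the filter.
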(event Custom|ReCheck
  (bind _textrender (Variables|Default|GetTextRender))
  (Variables|Default|SetQuestList (Variables|Default|GetSavedQuests))
  (Utilities|FlowControl|Sequence
    (:then_0
      (bind _output_get (Variables|Default|SetSavedQuests (Variables|Default|GetQuestList)))
      (for _array_element _output_get
        (bind _returnvalue (Utilities|GetDataTableRow "/Game/ThirdPerson/Blueprints/InteractionSystem/QuestSystem/Quest_DataTable.Quest_DataTable" (Utilities|String|StringToName (Utilities|String|EnumtoString _array_element)))
          (:then
            (bind _asplayer_bp (Utilities|Casting|CastToPlayer_BP (Game|GetPlayerCharacter 0)))
            (Variables|Default|SetPlayer_Ref _asplayer_bp)
            (for _array_element_2 (.Prerequisite (Utilities|Struct|BreakQuestInfo_S _returnvalue))
              (if (not (Utilities|Array|ContainsItem (Variables|/Game/ThirdPerson/Blueprints/Player_BP.Player_BP_C|GetCompletedQuests _asplayer_bp) _array_element_2))
                (Utilities|Array|RemoveItem (Variables|Default|GetQuestList) _array_element)
                (Development|PrintString "PreQuest not Met")))))))
    (:then_1
      (for _array_element_3 (Variables|/Game/ThirdPerson/Blueprints/Player_BP.Player_BP_C|GetCompletedQuests (Variables|Default|GetPlayer_Ref))
        (if (Utilities|Array|ContainsItem (Variables|Default|GetQuestList) _array_element_3)
          (Utilities|Array|RemoveItem (Variables|Default|GetQuestList) _array_element_3)
          (Utilities|Array|RemoveItem (Variables|Default|GetSavedQuests) _array_element_3)
          (Development|PrintString "Quest Removed")))
      (if (> (Utilities|Array|Length (Variables|Default|GetQuestList)) 0)
        (bind _output_get_2 (Variables|Default|SetValue "!"))
        (Rendering|Components|TextRender|SetText _textrender _output_get_2)
        (Rendering|SetVisibility _textrender true false)
        (CallFunction|Compare)
        (else
          (Rendering|SetVisibility _textrender false false))))))

(event Custom|Compare
  (for _array_element (Variables|Default|GetQuestList)
    (if (Utilities|Array|ContainsItem (Variables|/Game/ThirdPerson/Blueprints/Player_BP.Player_BP_C|GetAcceptedQuests (Variables|Default|GetPlayer_Ref)) _array_element)
      (bind _output_get (Variables|Default|SetValue "?"))
      (Rendering|Components|TextRender|SetText (Variables|Default|GetTextRender) _output_get)
      (Variables|Default|SetFound? true)))
  (if (not (Variables|Default|GetFound?))
    (bind _output_get_2 (Variables|Default|SetValue "!"))
    (Rendering|Components|TextRender|SetText (Variables|Default|GetTextRender) _output_get_2)))

(event EventBeginPlay
  (bind _textrender (Variables|Default|GetTextRender))
  (Utilities|FlowControl|Sequence
    (:then_0
      (bind _output_get (Variables|Default|SetSavedQuests (Variables|Default|GetQuestList)))
      (for _array_element _output_get
        (bind _returnvalue (Utilities|GetDataTableRow "/Game/ThirdPerson/Blueprints/InteractionSystem/QuestSystem/Quest_DataTable.Quest_DataTable" (Utilities|String|StringToName (Utilities|String|EnumtoString _array_element)))
          (:then
            (bind _asplayer_bp (Utilities|Casting|CastToPlayer_BP (Game|GetPlayerCharacter 0)))
            (Variables|Default|SetPlayer_Ref _asplayer_bp)
            (for _array_element_2 (.Prerequisite (Utilities|Struct|BreakQuestInfo_S _returnvalue))
              (if (not (Utilities|Array|ContainsItem (Variables|/Game/ThirdPerson/Blueprints/Player_BP.Player_BP_C|GetCompletedQuests _asplayer_bp) _array_element_2))
                (Utilities|Array|RemoveItem (Variables|Default|GetQuestList) _array_element)
                (Development|PrintString "PreQuest not Met")))))))
    (:then_1
      (for _array_element_3 (Variables|/Game/ThirdPerson/Blueprints/Player_BP.Player_BP_C|GetCompletedQuests (Variables|Default|GetPlayer_Ref))
        (if (Utilities|Array|ContainsItem (Variables|Default|GetQuestList) _array_element_3)
          (Utilities|Array|RemoveItem (Variables|Default|GetQuestList) _array_element_3)
          (Utilities|Array|RemoveItem (Variables|Default|GetSavedQuests) _array_element_3)
          (Development|PrintString "Quest Removed")))
      (if (> (Utilities|Array|Length (Variables|Default|GetQuestList)) 0)
        (bind _output_get_2 (Variables|Default|SetValue "!"))
        (Rendering|Components|TextRender|SetText _textrender _output_get_2)
        (Rendering|SetVisibility _textrender true false)
        (CallFunction|Compare)
        (else
          (Rendering|SetVisibility _textrender false false))))))

(event EventInteract
  (bind _returnvalue (Game|GetPlayerController 0))
  (bind _returnvalue_2 (Game|GetPlayerController 0))
  (if (Variables|Default|GetQuestScreenOpen?)
    (Widget|RemovefromParent (Variables|Default|GetQuestScreen))
    (Variables|Default|SetQuestScreenOpen? false)
    (Input|SetInputModeGameOnly _returnvalue_2)
    (Variables|/Script/Engine.PlayerController|SetbShowMouseCursor _returnvalue_2 false)
    (Variables|/Game/ThirdPerson/Blueprints/InteractionSystem/QuestSystem/QuestScreen_WBP.QuestScreen_WBP_C|SetHighlighted? (Variables|Default|GetQuestScreen) false)
    (bind _outactors (Actor|GetAllActorsOfClass "QuestGiver_BP_C"))
    (for _array_element _outactors
      (CallFunction|ReCheck _array_element))
    (else
      (Utilities|IsValid (Variables|Default|GetQuestScreen)
        (:Is%20Valid
          _)
        (:Is%20Not%20Valid
          (bind _returnvalue_3 (UserInterface|CreateWidget "/Game/ThirdPerson/Blueprints/InteractionSystem/QuestSystem/QuestScreen_WBP.QuestScreen_WBP_C" 0 self))
          (bind _output_get (Variables|Default|SetQuestScreen _returnvalue_3))))
      (UserInterface|Viewport|AddtoViewport _output_get 0)
      (Variables|Default|SetQuestScreenOpen? true)
      (Input|SetInputModeGameandUI _returnvalue _output_get "DoNotLock" true)
      (Variables|/Script/Engine.PlayerController|SetbShowMouseCursor _returnvalue true))))

(fn ConstructionScript
  (|CallParentFunction))