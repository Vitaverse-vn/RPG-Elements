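; Quest objective trigger volume that completes a find-type quest when the player enters it.
; On overlap by Player_BP, gated by a DoOnce that resets on exit, it checks whether the associated quest is among the player's accepted quests.
; It then finds that entry in the QuestLog, rewrites it with Completed set to true and prints a found message.
; The construction script sizes the box from BoxSize.
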(event OnComponentBeginOverlap(Box)
  (params (OverlappedComponent :type Primitive%20Component%20Object%20Reference) (OtherActor :type Actor%20Object%20Reference) (OtherComp :type Primitive%20Component%20Object%20Reference) (OtherBodyIndex :type Integer) (bFromSweep :type Boolean) (SweepResult :type Hit%20Result%20Structure%20%28by%20ref%29))
  (bind _asplayer_bp (Utilities|Casting|CastToPlayer_BP OtherActor))
  (Variables|Default|SetPlayer_Ref _asplayer_bp)
  (Utilities|FlowControl|DoOnce false
    (:Completed
      (if (Utilities|Array|ContainsItem (Variables|/Game/ThirdPerson/Blueprints/Player_BP.Player_BP_C|GetAcceptedQuests _asplayer_bp) (Variables|Default|GetQuestAssociated))
        (bind (_array_element _array_index) (Utilities|Array|ForEachLoopwithBreak (Variables|/Game/ThirdPerson/Blueprints/Player_BP.Player_BP_C|GetQuestLog (Variables|Default|GetPlayer_Ref)) :!label _label)
          (:LoopBody
            (if (Utilities|Enum|Equal(Enum) (.QuestID (Utilities|Struct|BreakQuestInfo_S _array_element)) (Variables|Default|GetQuestAssociated))
              (Variables|Default|SetQuestIDIndex _array_index)
              (Variables|Default|SetQuestInfoFound _array_element)
              (goto _label Break)))
          (:Completed
            (Utilities|Array|SetArrayElem (Variables|/Game/ThirdPerson/Blueprints/Player_BP.Player_BP_C|GetQuestLog (Variables|Default|GetPlayer_Ref)) (Variables|Default|GetQuestIDIndex) (Utilities|Struct|MakeQuestInfo_S (.QuestID (Utilities|Struct|BreakQuestInfo_S (Variables|Default|GetQuestInfoFound))) (.QuestType (Utilities|Struct|BreakQuestInfo_S (Variables|Default|GetQuestInfoFound))) (.QuestName (Utilities|Struct|BreakQuestInfo_S (Variables|Default|GetQuestInfoFound))) (.QuestDescription (Utilities|Struct|BreakQuestInfo_S (Variables|Default|GetQuestInfoFound))) (.Collectables (Utilities|Struct|BreakQuestInfo_S (Variables|Default|GetQuestInfoFound))) (.KillTargets (Utilities|Struct|BreakQuestInfo_S (Variables|Default|GetQuestInfoFound))) (.KillCount (Utilities|Struct|BreakQuestInfo_S (Variables|Default|GetQuestInfoFound))) (.Reward (Utilities|Struct|BreakQuestInfo_S (Variables|Default|GetQuestInfoFound))) (.Gold (Utilities|Struct|BreakQuestInfo_S (Variables|Default|GetQuestInfoFound))) (.XPReward (Utilities|Struct|BreakQuestInfo_S (Variables|Default|GetQuestInfoFound))) (.HasPrerequisite? (Utilities|Struct|BreakQuestInfo_S (Variables|Default|GetQuestInfoFound))) (.Prerequisite (Utilities|Struct|BreakQuestInfo_S (Variables|Default|GetQuestInfoFound))) true))
            (Development|PrintString "You found it!!")))))))

(event OnComponentEndOverlap(Box)
  (params (OverlappedComponent :type Primitive%20Component%20Object%20Reference) (OtherActor :type Actor%20Object%20Reference) (OtherComp :type Primitive%20Component%20Object%20Reference) (OtherBodyIndex :type Integer))
  (Utilities|Casting|CastToPlayer_BP OtherActor)
  (Utilities|FlowControl|DoOnce false) ; enters at Reset
)

(fn ConstructionScript
  (Components|Box|SetBoxExtent (Variables|Default|GetBox) (Variables|Default|GetBoxSize) true))