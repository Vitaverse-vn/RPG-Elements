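; BaseInteractable_BP is an interactable item that the player picks up.
; The construction script fills ItemInfo from the ItemsInfo_DataTB row named after the ItemName enum.
; Interact, when Interactable is set, passes ItemInfo to Player_BP's PickupItem and optionally destroys the actor.
; ElementalCheck stores an element type and attaches a Fire, Ice or Shock particle emitter to the Item component.
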(event EventInteract
  (if (Variables|Default|GetInteractable?)
    (bind _asplayer_bp (Utilities|Casting|CastToPlayer_BP (Game|GetPlayerCharacter 0)))
    (Default|PickupItem _asplayer_bp (Variables|Default|GetItem_Info))
    (if (Variables|Default|GetDestroy?)
      (Actor|DestroyActor))))

(fn ConstructionScript
  (bind _returnvalue (Utilities|GetDataTableRow "/Game/ThirdPerson/Blueprints/InteractionSystem/ItemsInfo_DataTB.ItemsInfo_DataTB" (Utilities|String|StringToName (Utilities|String|EnumtoString (Variables|Default|GetItem_Name))))
    (:then
      (Variables|Default|SetItem_Info _returnvalue))))

(fn ElementalCheck
  (params (ElementType :type ElementalTypes_E%20Enum :default "NewEnumerator0"))
  (bind _item (Variables|Default|GetItem))
  (bind _output_get (Variables|Default|SetElementalType ElementType))
  (switch Utilities|FlowControl|Switch|SwitchonElementalTypes_E _output_get
    (:NewEnumerator1
      (Effects|SpawnEmitterAttached "/Game/FXVarietyPack/Particles/P_ky_fireBall.P_ky_fireBall" _item "None" "0, 0, 0" "0, 0, 0" "1.000000,1.000000,1.000000" "SnapToTarget"))
    (:NewEnumerator2
      (Effects|SpawnEmitterAttached "/Game/FXVarietyPack/Particles/P_ky_waterBall.P_ky_waterBall" _item "None" "0, 0, 0" "0, 0, 0" "1.000000,1.000000,1.000000" "SnapToTarget"))
    (:NewEnumerator3
      (Effects|SpawnEmitterAttached "/Game/FXVarietyPack/Particles/P_ky_shootingStar1.P_ky_shootingStar1" _item "None" "0, 0, 0" "0, 0, 0" "1.000000,1.000000,1.000000" "SnapToTarget"))))