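; Shopkeeper NPC that toggles a shop screen on interaction and closes it when the player leaves its sphere.
; Opening fills the inventory from an item data table using expected-item enum names as row keys, then shows Shop_WBP with mouse input.
; The camera blends to the shopkeeper and hides the player while shopping, reversing on close.
; The construction script applies the mesh and selects an idle animation by NPC type.
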(event OnComponentEndOverlap(Sphere)
  (params (OverlappedComponent :type Primitive%20Component%20Object%20Reference) (OtherActor :type Actor%20Object%20Reference) (OtherComp :type Primitive%20Component%20Object%20Reference) (OtherBodyIndex :type Integer))
  (if (Variables|Default|GetShopOpen?)
    (Utilities|Casting|CastToPlayer_BP OtherActor)
    (CallFunction|ChecktheShop)))

(event Custom|ShowShop
  (bind _returnvalue (Game|GetPlayerController 0))
  (bind _returnvalue_2 (UserInterface|CreateWidget "/Game/ThirdPerson/Blueprints/InteractionSystem/ShopKeeper/Shop_WBP.Shop_WBP_C"))
  (Variables|/Game/ThirdPerson/Blueprints/InteractionSystem/ShopKeeper/Shop_WBP.Shop_WBP_C|SetShopKeeper_Ref _returnvalue_2 self)
  (bind _output_get (Variables|Default|SetShop_Ref _returnvalue_2))
  (UserInterface|Viewport|AddtoViewport _output_get 0)
  (Input|SetInputModeGameandUI _returnvalue _output_get "DoNotLock" true)
  (Variables|/Script/Engine.PlayerController|SetbShowMouseCursor _returnvalue true)
  (Variables|Default|SetShopOpen? true))

(event Custom|CheckTheShop
  (bind _returnvalue (Game|GetPlayerController 0))
  (bind _inventoryexpected (Variables|Default|GetInventoryExpected))
  (if (Variables|Default|GetShopOpen?)
    (Widget|RemovefromParent (Variables|Default|GetShop_Ref))
    (Input|SetInputModeGameOnly _returnvalue)
    (Variables|/Script/Engine.PlayerController|SetbShowMouseCursor _returnvalue false)
    (Variables|Default|SetShopOpen? false)
    (Game|Player|SetViewTargetwithBlend (Game|GetPlayerController 0) (Game|Player|GetPlayerPawn 0) 0.5 "VTBlend_Linear" 0.0 false)
    (bind _asplayer_bp (Utilities|Casting|CastToPlayer_BP (Game|GetPlayerCharacter 0)))
    (Rendering|SetActorHiddenInGame _asplayer_bp false)
    (else
      (for _index (range 0 (- (Utilities|Array|Length _inventoryexpected) 1))
        (bind _returnvalue_2 (Utilities|GetDataTableRow "/Game/ThirdPerson/Blueprints/InteractionSystem/ItemsInfo_DataTB.ItemsInfo_DataTB" (Utilities|String|StringToName (Utilities|String|EnumtoString (Utilities|Array|Get(acopy) _inventoryexpected _index))))
          (:then
            (Utilities|Array|AddUnique (Variables|Default|GetInventory) _returnvalue_2)
            (Game|Player|SetViewTargetwithBlend (Game|GetPlayerController 0) self 0.5 "VTBlend_Linear" 0.0 false)
            (bind _asplayer_bp_2 (Utilities|Casting|CastToPlayer_BP (Game|GetPlayerCharacter 0)))
            (Rendering|SetActorHiddenInGame _asplayer_bp_2 true))))
      (CallFunction|ShowShop))))

(event EventBeginPlay)

(event Collision|EventActorBeginOverlap
  (params (OtherActor :type Actor%20Object%20Reference)))

(event EventTick
  (params (DeltaSeconds :type Float%20%28single-precision%29)))

(event EventInteract
  (bind _returnvalue (Game|GetPlayerController 0))
  (bind _inventoryexpected (Variables|Default|GetInventoryExpected))
  (if (Variables|Default|GetShopOpen?)
    (Widget|RemovefromParent (Variables|Default|GetShop_Ref))
    (Input|SetInputModeGameOnly _returnvalue)
    (Variables|/Script/Engine.PlayerController|SetbShowMouseCursor _returnvalue false)
    (Variables|Default|SetShopOpen? false)
    (Game|Player|SetViewTargetwithBlend (Game|GetPlayerController 0) (Game|Player|GetPlayerPawn 0) 0.5 "VTBlend_Linear" 0.0 false)
    (bind _asplayer_bp (Utilities|Casting|CastToPlayer_BP (Game|GetPlayerCharacter 0)))
    (Rendering|SetActorHiddenInGame _asplayer_bp false)
    (else
      (for _index (range 0 (- (Utilities|Array|Length _inventoryexpected) 1))
        (bind _returnvalue_2 (Utilities|GetDataTableRow "/Game/ThirdPerson/Blueprints/InteractionSystem/ItemsInfo_DataTB.ItemsInfo_DataTB" (Utilities|String|StringToName (Utilities|String|EnumtoString (Utilities|Array|Get(acopy) _inventoryexpected _index))))
          (:then
            (Utilities|Array|AddUnique (Variables|Default|GetInventory) _returnvalue_2)
            (Game|Player|SetViewTargetwithBlend (Game|GetPlayerController 0) self 0.5 "VTBlend_Linear" 0.0 false)
            (bind _asplayer_bp_2 (Utilities|Casting|CastToPlayer_BP (Game|GetPlayerCharacter 0)))
            (Rendering|SetActorHiddenInGame _asplayer_bp_2 true))))
      (CallFunction|ShowShop))))

(fn ConstructionScript
  (bind _skeletalmesh (Variables|Default|GetSkeletalMesh))
  (|CallParentFunction)
  (Class|SkinnedMeshComponent|SetSkeletalMesh _skeletalmesh (Variables|Default|GetMesh) true)
  (Components|Animation|OverrideAnimationData _skeletalmesh (Utilities|Select :Index (Variables|Default|GetNPCType) :NewEnumerator0 "/Game/ThirdPerson/Blueprints/Characters/NPC/GMFemale/ConsumptionShop_Dwarf_Idle.ConsumptionShop_Dwarf_Idle" :NewEnumerator1 0 :NewEnumerator2 0 :NewEnumerator3 "/Game/ThirdPerson/Blueprints/Characters/NPC/EquipmentVendor/GearsShop_Sad_Idle.GearsShop_Sad_Idle" :NewEnumerator4 "/Game/ThirdPerson/Blueprints/Characters/NPC/MagicTeacher/IdleMagicSensei.IdleMagicSensei") true true 0.0 1.0))