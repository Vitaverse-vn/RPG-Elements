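; Base Blueprint for a harvestable actor that yields items to the player when it takes damage.
; Each damage event lowers Health by one, regardless of damage amount, then calls PickupItem with its ItemInfo a random number of times on player 0's Player_BP.
; The actor destroys itself after granting the final batch when Health reaches zero.
; Items go to that player whoever dealt the damage.
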(event Game|Damage|EventAnyDamage
  (params (Damage :type Float%20%28single-precision%29) (DamageType :type Damage%20Type%20Object%20Reference) (InstigatedBy :type Controller%20Object%20Reference) (DamageCauser :type Actor%20Object%20Reference))
  (bind _result (Math|Integer|DecrementInt (Variables|Default|GetHealth))
    (:%20%20
      (if (<= _result 0)
        (bind _asplayer_bp (Utilities|Casting|CastToPlayer_BP (Game|GetPlayerCharacter 0)))
        (for _index (range 0 (Math|Random|RandomIntegerinRange 3 5))
          (Default|PickupItem _asplayer_bp (Variables|Default|GetItem_Info)))
        (Actor|DestroyActor)
        (else
          (bind _asplayer_bp_2 (Utilities|Casting|CastToPlayer_BP (Game|GetPlayerCharacter 0)))
          (for _index_2 (range 0 (Math|Random|RandomIntegerinRange 3 5))
            (Default|PickupItem _asplayer_bp_2 (Variables|Default|GetItem_Info))))))))

(fn ConstructionScript
  (|CallParentFunction))