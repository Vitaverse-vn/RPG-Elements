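; WoodArrow_BP is an arrow projectile that damages actors tagged "Enemy" when its Box collision overlaps them.
; On a hit it sends the target a hurt message, then adds a fire or ice message according to its ElementalType.
; All element types then apply ArrowDamage with player character 0 as damage causer, print the damage value and destroy the arrow.
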(event OnComponentBeginOverlap(Box)
  (params (OverlappedComponent :type Primitive%20Component%20Object%20Reference) (OtherActor :type Actor%20Object%20Reference) (OtherComp :type Primitive%20Component%20Object%20Reference) (OtherBodyIndex :type Integer) (bFromSweep :type Boolean) (SweepResult :type Hit%20Result%20Structure%20%28by%20ref%29))
  (bind _arrowdamage (Variables|Default|GetArrowDamage))
  (if (Actor|ActorHasTag OtherActor "Enemy")
    (Class|HurtBPI|Hurt(Message) OtherActor)
    (switch Utilities|FlowControl|Switch|SwitchonElementalTypes_E (Variables|Default|GetElementalType)
      (:NewEnumerator0
        _)
      (:NewEnumerator1
        (Class|StatusFXBPI|Fire(Message) OtherActor))
      (:NewEnumerator2
        (Class|StatusFXBPI|Ice(Message) OtherActor)))
    (Game|Damage|ApplyDamage OtherActor _arrowdamage 0 (Game|GetPlayerCharacter 0))
    (Development|PrintString (Utilities|String|ToString(Float) _arrowdamage))
    (Actor|DestroyActor)))

(event EventBeginPlay)

(event Collision|EventActorBeginOverlap
  (params (OtherActor :type Actor%20Object%20Reference)))

(event EventTick
  (params (DeltaSeconds :type Float%20%28single-precision%29)))

(fn ConstructionScript
  (|CallParentFunction))