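; Magic teacher NPC that opens a spell shop when the player interacts with it.
; Opening fills SpellInventory from Spells_DataTB using SpellsExpected, creates MagicShop_WBP, blends the camera to the NPC, hides the player and enables UI input.
; Interacting again or leaving the Sphere overlap closes the shop and restores the player's view and controls.
; The construction script sets the skeletal mesh and picks an idle animation by NPCType.
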(event OnComponentEndOverlap(Sphere)
  (params (OverlappedComponent :type Primitive%20Component%20Object%20Reference) (OtherActor :type Actor%20Object%20Reference) (OtherComp :type Primitive%20Component%20Object%20Reference) (OtherBodyIndex :type Integer))
  (if (Variables|Default|GetMagicShopOpen?)
    (Utilities|Casting|CastToPlayer_BP OtherActor)
    (CallFunction|CheckMagicShop)))

(event Custom|ShowMagicShop
  (bind _returnvalue (Game|GetPlayerController 0))
  (bind _returnvalue_2 (UserInterface|CreateWidget "/Game/ThirdPerson/Blueprints/InteractionSystem/MagicTeacher/MagicShop_WBP.MagicShop_WBP_C"))
  (Variables|Default|SetMagicShop_Ref _returnvalue_2)
  (Variables|/Game/ThirdPerson/Blueprints/InteractionSystem/MagicTeacher/MagicShop_WBP.MagicShop_WBP_C|SetMagicTeacher_Ref _returnvalue_2 self)
  (UserInterface|Viewport|AddtoViewport _returnvalue_2 0)
  (Game|Player|SetViewTargetwithBlend _returnvalue self 0.5 "VTBlend_Linear" 0.0 false)
  (Input|SetInputModeGameandUI _returnvalue (Variables|Default|GetMagicShop_Ref) "DoNotLock" true)
  (Variables|/Script/Engine.PlayerController|SetbShowMouseCursor _returnvalue true)
  (bind _asplayer_bp (Utilities|Casting|CastToPlayer_BP (Game|GetPlayerCharacter 0)))
  (Rendering|SetActorHiddenInGame _asplayer_bp true))

(event Custom|CheckMagicShop
  (bind _returnvalue (Game|GetPlayerController 0))
  (bind _spellsexpected (Variables|Default|GetSpellsExpected))
  (if (Variables|Default|GetMagicShopOpen?)
    (Widget|RemovefromParent (Variables|Default|GetMagicShop_Ref))
    (Variables|Default|SetMagicShopOpen? false)
    (Game|Player|SetViewTargetwithBlend _returnvalue (Game|Player|GetPlayerPawn 0) 0.5 "VTBlend_Linear" 0.0 false)
    (Input|SetInputModeGameOnly _returnvalue)
    (Variables|/Script/Engine.PlayerController|SetbShowMouseCursor _returnvalue false)
    (bind _asplayer_bp (Utilities|Casting|CastToPlayer_BP (Game|GetPlayerCharacter 0)))
    (Rendering|SetActorHiddenInGame _asplayer_bp false)
    (else
      (for _index (range 0 (- (Utilities|Array|Length _spellsexpected) 1))
        (bind _returnvalue_2 (Utilities|GetDataTableRow "/Game/ThirdPerson/Blueprints/MagicSystem/Spells_DataTB.Spells_DataTB" (Utilities|String|StringToName (Utilities|String|EnumtoString (Utilities|Array|Get(acopy) _spellsexpected _index))))
          (:then
            (Utilities|Array|AddUnique (Variables|Default|GetSpellInventory) _returnvalue_2))))
      (CallFunction|ShowMagicShop)
      (Variables|Default|SetMagicShopOpen? true))))

(event EventInteract
  (bind _returnvalue (Game|GetPlayerController 0))
  (bind _spellsexpected (Variables|Default|GetSpellsExpected))
  (if (Variables|Default|GetMagicShopOpen?)
    (Widget|RemovefromParent (Variables|Default|GetMagicShop_Ref))
    (Variables|Default|SetMagicShopOpen? false)
    (Game|Player|SetViewTargetwithBlend _returnvalue (Game|Player|GetPlayerPawn 0) 0.5 "VTBlend_Linear" 0.0 false)
    (Input|SetInputModeGameOnly _returnvalue)
    (Variables|/Script/Engine.PlayerController|SetbShowMouseCursor _returnvalue false)
    (bind _asplayer_bp (Utilities|Casting|CastToPlayer_BP (Game|GetPlayerCharacter 0)))
    (Rendering|SetActorHiddenInGame _asplayer_bp false)
    (else
      (for _index (range 0 (- (Utilities|Array|Length _spellsexpected) 1))
        (bind _returnvalue_2 (Utilities|GetDataTableRow "/Game/ThirdPerson/Blueprints/MagicSystem/Spells_DataTB.Spells_DataTB" (Utilities|String|StringToName (Utilities|String|EnumtoString (Utilities|Array|Get(acopy) _spellsexpected _index))))
          (:then
            (Utilities|Array|AddUnique (Variables|Default|GetSpellInventory) _returnvalue_2))))
      (CallFunction|ShowMagicShop)
      (Variables|Default|SetMagicShopOpen? true))))

(fn ConstructionScript
  (bind _skeletalmesh (Variables|Default|GetSkeletalMesh))
  (|CallParentFunction)
  (Class|SkinnedMeshComponent|SetSkeletalMesh _skeletalmesh (Variables|Default|GetMesh) true)
  (Components|Animation|OverrideAnimationData _skeletalmesh (Utilities|Select :Index (Variables|Default|GetNPCType) :NewEnumerator0 "/Game/ThirdPerson/Blueprints/Characters/NPC/GMFemale/ConsumptionShop_Dwarf_Idle.ConsumptionShop_Dwarf_Idle" :NewEnumerator1 0 :NewEnumerator2 0 :NewEnumerator3 "/Game/ThirdPerson/Blueprints/Characters/NPC/EquipmentVendor/GearsShop_Sad_Idle.GearsShop_Sad_Idle" :NewEnumerator4 "/Game/ThirdPerson/Blueprints/Characters/NPC/MagicTeacher/IdleMagicSensei.IdleMagicSensei") true true 0.0 1.0))